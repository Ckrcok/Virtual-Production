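; A combination wrench pickup actor that gives the player a wrench.
; When the player pawn begins overlapping the Sphere component, it prints a debug string, sets HasWrench on the ThirdPersonCharacter and destroys itself.
; A WrenchAnimation timeline is wired to spin the static mesh through yaw, but nothing in the graph triggers it.
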(event `self.Sphere.OnComponentBeginOverlap`
  (params (OverlappedComponent :type "PrimitiveComponent Object Reference") (OtherActor :type "Actor Object Reference") (OtherComp :type "PrimitiveComponent Object Reference") (OtherBodyIndex :type Integer) (bFromSweep :type Boolean) (SweepResult :type "HitResult Structure (by ref)"))
  (bind _returnvalue (`GameplayStatics.GetPlayerPawn` 0))
  (bind _output_get (set `self.Player` _returnvalue))
  (if (== OtherActor _output_get)
    (`KismetSystemLibrary.PrintString` "PickupWrench")
    (bind _asthird_person_character (cast `/Game/ThirdPersonBP/Blueprints/ThirdPersonCharacter` _returnvalue))
    (set `/Game/ThirdPersonBP/Blueprints/ThirdPersonCharacter.HasWrench` true _asthird_person_character)
    (`self.K2_DestroyActor`)))

(fn `UserConstructionScript`)